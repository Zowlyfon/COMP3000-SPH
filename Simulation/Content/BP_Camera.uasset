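; BP_Camera is a player-controlled spring arm camera that rotates and zooms from axis inputs.
; RotateLeft and RotateUp feed controller yaw and pitch input.
; ZoomIn adds its raw axis value to the spring arm's target length, with no clamping or delta-time scaling.
; BeginPlay saves the initial arm length in SpringArmLength, which this graph never reads back.
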(event `InputAxis|ZoomIn`
  (params (AxisValue :type "Float (single-precision)"))
  (bind _springarm (`self.SpringArm`))
  (set `SpringArmComponent.TargetArmLength` (+ AxisValue (`SpringArmComponent.TargetArmLength` _springarm)) _springarm))

(event `InputAxis|RotateLeft`
  (params (AxisValue :type "Float (single-precision)"))
  (`self.AddControllerYawInput` AxisValue))

(event `self.ReceiveBeginPlay`
  (set `self.SpringArmLength` (`SpringArmComponent.TargetArmLength` (`self.SpringArm`))))

(event `InputAxis|RotateUp`
  (params (AxisValue :type "Float (single-precision)"))
  (`self.AddControllerPitchInput` AxisValue))

(fn `UserConstructionScript`)